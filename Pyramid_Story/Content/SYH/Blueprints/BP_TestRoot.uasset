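; BP_TestRoot is a trigger actor that shows the WBP_Select2 selection UI when the player comes near.
; It caches the BP_SYHPlayer pawn on BeginPlay, then on Box overlap checks the class and a short distance from the actor.
; The Show flag limits display to one time, though the widget is created before that check.
; Displaying it also enables the mouse cursor, mouse-over events and Game-and-UI input.
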(event OnComponentBeginOverlap(Box)
  (params (OverlappedComponent :type Primitive%20Component%20Object%20Reference) (OtherActor :type Actor%20Object%20Reference) (OtherComp :type Primitive%20Component%20Object%20Reference) (OtherBodyIndex :type Integer) (bFromSweep :type Boolean) (SweepResult :type Hit%20Result%20Structure%20%28by%20ref%29))
  (bind _returnvalue (Game|GetPlayerController 0))
  ;[1 1 1] box collision과 부딪히면서 특정 리내에 존재하면 UI띄우기
  (if (Class|GameplayStatics|ObjectIsA OtherActor "/Game/SYH/Blueprints/BP_SYHPlayer.BP_SYHPlayer_C")
    (Utilities|IsValid OtherActor
      (:Is%20Valid
        (if (<= (Math|Vector|VectorLength (- (Transformation|GetActorLocation) (Transformation|GetActorLocation (Variables|Default|GetAs%20BP%20SYHPlayer)))) 2e+02)
          (bind _returnvalue_2 (UserInterface|CreateWidget "/Game/YWK/WIdget/WBP_Select2.WBP_Select2_C"))
          (if (Variables|Default|GetShow)
            (UserInterface|Viewport|AddtoViewport _returnvalue_2 0)
            ;[1 1 1] 마우스 커서 띄우기
            (Variables|/Script/Engine.PlayerController|SetbShowMouseCursor _returnvalue true)
            (Variables|/Script/Engine.PlayerController|SetbEnableMouseOverEvents _returnvalue true)
            (Variables|Default|SetShow false)
            (Input|SetInputModeGameandUI _returnvalue 0 "DoNotLock" true false)))))))

(event EventBeginPlay
  ;[1 1 1] player cast
  (bind _asbp_syhplayer (Utilities|Casting|CastToBP_SYHPlayer (Game|Player|GetPlayerPawn 0)))
  (Variables|Default|SetAs%20BP%20SYHPlayer _asbp_syhplayer))

(event Collision|EventActorBeginOverlap
  (params (OtherActor :type Actor%20Object%20Reference)))

(event EventTick
  (params (DeltaSeconds :type Float%20%28single-precision%29)))

(fn ConstructionScript)