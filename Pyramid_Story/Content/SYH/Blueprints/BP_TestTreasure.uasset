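; BP_TestTreasure is a test treasure (relic) actor that shows UI as the player approaches or hovers the cursor over it.
; It caches BP_SYHPlayer on BeginPlay for distance checks.
; Box overlap shows a fading WBP_beforeSelect2 prompt when the player is near; its removal code is unconnected.
; Hovering at closer range shows WBP_Test, guarded by the Make flag, and cursor exit removes it through GetAllWidgetsOfClass.
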(event OnComponentBeginOverlap(Box)
  (params (OverlappedComponent :type Primitive%20Component%20Object%20Reference) (OtherActor :type Actor%20Object%20Reference) (OtherComp :type Primitive%20Component%20Object%20Reference) (OtherBodyIndex :type Integer) (bFromSweep :type Boolean) (SweepResult :type Hit%20Result%20Structure%20%28by%20ref%29))
  (bind _returnvalue (UserInterface|CreateWidget "/Game/SYH/Blueprints/WBP_beforeSelect2.WBP_beforeSelect2_C"))
  (if (<= (Math|Vector|VectorLength (- (Transformation|GetActorLocation) (Transformation|GetActorLocation (Variables|Default|GetAs%20BP%20SYHPlayer)))) 3e+02)
    (UserInterface|Viewport|AddtoViewport _returnvalue 0)
    (Default|PlayFade _returnvalue)))

(event EventBeginPlay
  (bind _asbp_syhplayer (Utilities|Casting|CastToBP_SYHPlayer (Game|Player|GetPlayerPawn 0)))
  (Variables|Default|SetAs%20BP%20SYHPlayer _asbp_syhplayer))

(event Collision|EventActorBeginOverlap
  (params (OtherActor :type Actor%20Object%20Reference)))

(event EventTick
  (params (DeltaSeconds :type Float%20%28single-precision%29)))

(event MouseInput|EventActorEndCursorOver
  ;[1 1 1] cursor를 떼면 UI 사라짐
  (if (Variables|Default|GetMake)
    (bind _foundwidgets (Widget|GetAllWidgetsOfClass "/Game/SYH/Blueprints/WBP_Test.WBP_Test_C" true))
    (Widget|RemovefromParent _foundwidgets)
    (Variables|Default|SetMake false)))

(event MouseInput|EventActorBeginCursorOver
  ;[1 1 1] cursor를 유물 위에 올리면 UI 뜸
  (if (not (Variables|Default|GetMake))
    (bind _returnvalue (UserInterface|CreateWidget "/Game/SYH/Blueprints/WBP_Test.WBP_Test_C"))
    (if (<= (Math|Vector|VectorLength (- (Transformation|GetActorLocation) (Transformation|GetActorLocation (Variables|Default|GetAs%20BP%20SYHPlayer)))) 1.5e+02)
      (UserInterface|Viewport|AddtoViewport _returnvalue 1)
      (Variables|Default|SetMake true))))

(fn ConstructionScript)