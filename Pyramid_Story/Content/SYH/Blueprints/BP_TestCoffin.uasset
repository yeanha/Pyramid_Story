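; BP_TestCoffin is a coffin actor that shows a selection UI when the player approaches and slides forward when opened.
; Box overlap by BP_SYHPlayer within a set distance creates WBP_Select3, adding it to the viewport only once with mouse cursor and Game-and-UI input.
; OpenCoffin starts movement along the forward vector in Tick.
; A frame counter, not elapsed time, removes the widget early in the slide and later stops it.
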(event OnComponentBeginOverlap(Box)
  (params (OverlappedComponent :type Primitive%20Component%20Object%20Reference) (OtherActor :type Actor%20Object%20Reference) (OtherComp :type Primitive%20Component%20Object%20Reference) (OtherBodyIndex :type Integer) (bFromSweep :type Boolean) (SweepResult :type Hit%20Result%20Structure%20%28by%20ref%29))
  (bind _returnvalue (Game|GetPlayerController 0))
  ;[1 1 1] box collision과 부딪히면서 특정 리내에 존재하면 UI띄우기
  (if (Class|GameplayStatics|ObjectIsA OtherActor "/Game/SYH/Blueprints/BP_SYHPlayer.BP_SYHPlayer_C")
    (if (<= (Math|Vector|VectorLength (- (Transformation|GetActorLocation) (Transformation|GetActorLocation (Variables|Default|GetAs%20BP%20SYHPlayer)))) 6e+02)
      (bind _returnvalue_2 (UserInterface|CreateWidget "/Game/YWK/WIdget/WBP_Select3.WBP_Select3_C"))
      (if (Variables|Default|GetShow)
        (UserInterface|Viewport|AddtoViewport _returnvalue_2 0)
        ;[1 1 1] 마우스 커서 띄우기
        (Variables|/Script/Engine.PlayerController|SetbShowMouseCursor _returnvalue true)
        (Variables|/Script/Engine.PlayerController|SetbEnableMouseOverEvents _returnvalue true)
        (Variables|Default|SetShow false)
        (Input|SetInputModeGameandUI _returnvalue 0 "DoNotLock" true false)))))

(event Collision|EventActorBeginOverlap
  (params (OtherActor :type Actor%20Object%20Reference)))

(event EventTick
  (params (DeltaSeconds :type Float%20%28single-precision%29))
  (if (Variables|Default|GetIsMove)
    (Transformation|SetActorLocation (+ (Transformation|GetActorLocation) (* (Transformation|GetActorForwardVector) (Variables|Default|GetSpeed) DeltaSeconds)) false false)
    (bind _output_get (Variables|Default|SetCount (+ (Variables|Default|GetCount) 1.0)))
    (if (== _output_get 5e+01)
      (bind _foundwidgets (Widget|GetAllWidgetsOfClass "/Game/YWK/WIdget/WBP_Select3.WBP_Select3_C" true))
      (Widget|RemovefromParent _foundwidgets))
    (if (>= _output_get 4e+02)
      (Variables|Default|SetIsMove false))))

(event EventBeginPlay
  ;[1 1 1] player cast
  (bind _asbp_syhplayer (Utilities|Casting|CastToBP_SYHPlayer (Game|Player|GetPlayerPawn 0)))
  (Variables|Default|SetAs%20BP%20SYHPlayer _asbp_syhplayer))

(fn ConstructionScript)

(fn OpenCoffin
  (params (DeltaTime :type Float%20%28double-precision%29))
  (Variables|Default|SetIsMove true))